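; Base Character for combat-level units, exposing health, damage, effects, faction, simple movement and selection UI functions.
; Damage and effect components do the work, with damage events bound in the construction script to update the health and abilities bars.
; The health bar shows on hover or while selected, using a looping timer instead of Tick to face the camera.
; Death ragdolls the mesh, then after a delay randomly destroys or fully revives the unit.
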(event `self.ReceiveBeginPlay`
  (`self.InitHealthBar`))

(event `UpdateHealthBarWidgetRotation`
  (bind _healthbar (`self.HealthBar`))
  ;[1 1 1] Ensures actors health bar is always facing camera
  (`SceneComponent.K2_SetWorldRotation` _healthbar (`KismetMathLibrary.FindLookAtRotation` (`SceneComponent.K2_GetComponentLocation` _healthbar) (`SceneComponent.K2_GetComponentLocation` (`PlayerCameraManager.TransformComponent` (`GameplayStatics.GetPlayerCameraManager` 0)))) false false))

(event `On Death`
  (bind _mesh (`self.Mesh`))
  ;[1 1 1] Saves the meshes transform incase of revive... then enables ragdol and collision, hides some UI elements before going into a 5 sec wait... in the end, a 50% chance of death vs revive
  (`CharacterMovementComponent.DisableMovement` (`self.CharacterMovement`))
  (set `self.MeshTransformCache` (`SceneComponent.K2_GetComponentToWorld` (`self.Mesh`)))
  (`PrimitiveComponent.SetSimulatePhysics` _mesh true)
  (`PrimitiveComponent.SetCollisionEnabled` _mesh "QueryAndPhysics")
  (`/Game/ASE/CombatLevel/CommandSystem/BPI_Commandable.HideHealthBar`)
  (`/Game/ASE/CombatLevel/CommandSystem/BPI_Commandable.HideAbilities`)
  (`/Game/ASE/CombatLevel/CommandSystem/BPI_Commandable.HideSelectedIndicator`)
  (`KismetSystemLibrary.Delay` 5.0)
  (if (`KismetMathLibrary.RandomBool`)
    (`self.K2_DestroyActor`)
    (else
      (`self.On Revive`))))

(event `On Revive`
  (bind _bpc_damagesystem (`self.BPC_DamageSystem`))
  (bind _mesh (`self.Mesh`))
  ;[1 1 1] Revives Actor with 100% HP
  (`PrimitiveComponent.SetSimulatePhysics` _mesh false)
  (`PrimitiveComponent.SetCollisionEnabled` _mesh "NoCollision")
  (`SceneComponent.K2_SetWorldTransform` _mesh (`self.MeshTransformCache`) true false)
  (`CharacterMovementComponent.SetMovementMode` (`self.CharacterMovement`) "MOVE_Walking" 0)
  (set `/Game/ASE/CombatLevel/DamageSystem/BPC_DamageSystem.IsDead` false _bpc_damagesystem)
  (`self.HealByValue` (`/Game/ASE/CombatLevel/DamageSystem/BPC_DamageSystem.MaxHealth` _bpc_damagesystem)))

(event `On Attack Updated`
  (bind _abilitiesbarref (`self.AbilitiesBarRef`))
  ;[1 1 1] Called when damage system component update attack listener is called, will update unit stats displayed to UI
  (`/Engine/EditorBlueprintResources/StandardMacros.IsValid` _abilitiesbarref
    (:`Is Valid`
      (`/Game/ASE/CombatLevel/UI/UWB_UnitAbilitiesBar.Update Attack` _abilitiesbarref (`/Game/ASE/CombatLevel/DamageSystem/BPC_DamageSystem.Attack` (`self.BPC_DamageSystem`))))))

(event `On Health Updated`
  (bind _healthbarref (`self.HealthBarRef`))
  (bind _abilitiesbarref (`self.AbilitiesBarRef`))
  ;[1 1 1] Updating Health bar and Abilities bar widgets when health is updated (only if visible and valid)
  (`|ExecutionSequence`
    (:`then_0`
      (`/Engine/EditorBlueprintResources/StandardMacros.IsValid` _abilitiesbarref
        (:`Is Valid`
          (`/Game/ASE/CombatLevel/UI/UWB_UnitAbilitiesBar.UpdateHealth` _abilitiesbarref (`/Game/ASE/CombatLevel/DamageSystem/BPC_DamageSystem.Health` (`self.BPC_DamageSystem`))))))
    (:`then_1`
      (if (`Widget.IsVisible` _healthbarref)
        (`/Game/ASE/CombatLevel/UI/UWB_UnitHealthBar.UpdateHealth` _healthbarref (`/Game/ASE/CombatLevel/DamageSystem/BPC_DamageSystem.Health` (`self.BPC_DamageSystem`)))))))

(event `self.CapsuleComponent.OnBeginCursorOver`
  (params (TouchedComponent :type "PrimitiveComponent Object Reference"))
  ;[1 1 1] On Hovered, if health bar is not visible, call the show health bar function
  (if (not (`SceneComponent.IsVisible` (`self.HealthBar`)))
    (`self.ShowHealthBar`)))

(event `self.CapsuleComponent.OnEndCursorOver`
  (params (TouchedComponent :type "PrimitiveComponent Object Reference"))
  ;[1 1 1] On unhovered, if unit is selected, dont do anything, else call the hide health bar function
  (if (not (`SceneComponent.IsVisible` (`self.SelectionIndicatorDecal`)))
    (`self.HideHealthBar`)))

(event `On Damage Response`
  (params (ResponseType :type "/Game/ASE/CombatLevel/DamageSystem/E_DamageResponseType Enum" :default "NewEnumerator0")))

(event `On Damage Blocked`)

(fn `ApplyEffect`
  (params (Effect :type "/Game/ASE/CombatLevel/EffectSystem/S_Effect Structure"))
  (returns (Result :type "/Game/ASE/CombatLevel/EffectSystem/E_ApplyEffectResult Enum") (EffectRef :type "/Game/ASE/CombatLevel/EffectSystem/Effects/BPC_Effect_Base Object Reference"))
  (bind (_result _effectref) (`/Game/ASE/CombatLevel/EffectSystem/BPI_Effectable.ApplyEffect` (`self.BPC_EffectManager`) Effect))
  (return _result _effectref))

(fn `GetCurrentHealth`
  (returns (Health :type "Float (double-precision)"))
  (return (`/Game/ASE/CombatLevel/DamageSystem/BPC_DamageSystem.Health` (`self.BPC_DamageSystem`))))

(fn `GetFaction`
  (returns (UnitsFaction :type "/Game/ASE/CombatLevel/CommandSystem/E_Faction Enum"))
  (return (`self.EFaction`)))

(fn `GetMaxHealth`
  (returns (MaxHealth :type "Float (double-precision)"))
  (return (`/Game/ASE/CombatLevel/DamageSystem/BPC_DamageSystem.MaxHealth` (`self.BPC_DamageSystem`))))

(fn `GetUnitType`
  (returns (IsBuilding :type Boolean))
  (return false))

(fn `HealByValue`
  (params (HealAmount :type "Float (double-precision)"))
  (returns (NewHealth :type "Float (double-precision)"))
  (bind _newhealth (`/Game/ASE/CombatLevel/DamageSystem/BPC_DamageSystem.Heal` (`self.BPC_DamageSystem`) HealAmount))
  (return _newhealth))

(fn `HideAbilities`
  (returns (WasSuccessful :type Boolean))
  (bind _abilitiesbarref (`self.AbilitiesBarRef`))
  (`/Engine/EditorBlueprintResources/StandardMacros.IsValid` _abilitiesbarref
    (:`Is Valid`
      (`Widget.RemoveFromParent` _abilitiesbarref)
      (set `self.AbilitiesBarRef` null)
      (return true))
    (:`Is Not Valid`
      (return false))))

(fn `HideHealthBar`
  (returns (WasSuccessful :type Boolean))
  (`SceneComponent.SetVisibility` (`self.HealthBar`) false false)
  (`KismetSystemLibrary.K2_ClearAndInvalidateTimerHandle` (`self.HBRoationTickTimerRef`))
  (return true))

(fn `HideSelectedIndicator`
  (returns (WasSuccessful :type Boolean))
  (bind _selectionindicatordecal (`self.SelectionIndicatorDecal`))
  (`SceneComponent.SetVisibility` _selectionindicatordecal false false)
  (`ActorComponent.Deactivate` _selectionindicatordecal)
  (return true))

(fn `InitHealthBar`
  (bind _bpc_damagesystem (`self.BPC_DamageSystem`))
  (bind _asuwb_unit_health_bar (cast `/Game/ASE/CombatLevel/UI/UWB_UnitHealthBar` (`WidgetComponent.GetUserWidgetObject` (`self.HealthBar`))))
  (bind _output_get (set `self.HealthBarRef` _asuwb_unit_health_bar))
  (`/Game/ASE/CombatLevel/UI/UWB_UnitHealthBar.UpdateHealth` _output_get (`/Game/ASE/CombatLevel/DamageSystem/BPC_DamageSystem.Health` _bpc_damagesystem))
  (`/Game/ASE/CombatLevel/UI/UWB_UnitHealthBar.UpdateMaxHealth` _output_get (`/Game/ASE/CombatLevel/DamageSystem/BPC_DamageSystem.MaxHealth` _bpc_damagesystem)))

(fn `MoveToLocation`
  (params (Destination :type "Vector Structure"))
  (returns (WasSuccessful :type Boolean))
  (`AIBlueprintHelperLibrary.SimpleMoveToLocation` (`self.GetController`) Destination)
  (return true))

(fn `ShowAbilities`
  (returns (WasSuccessful :type Boolean))
  (if (not (`/Game/ASE/CombatLevel/DamageSystem/BPC_DamageSystem.IsDead` (`self.BPC_DamageSystem`)))
    (bind _returnvalue (`|CreateWidget` "/Game/ASE/CombatLevel/UI/UWB_UnitAbilitiesBar.UWB_UnitAbilitiesBar_C" (`GameplayStatics.GetPlayerController` 0)))
    (bind _output_get (set `self.AbilitiesBarRef` _returnvalue))
    (`/Engine/EditorBlueprintResources/StandardMacros.IsValid` _output_get
      (:`Is Valid`
        (`self.UpdateAllAbilitiesInfo` _returnvalue)
        (`UserWidget.AddToViewport` _returnvalue 5)
        (`WidgetBlueprintLibrary.SetInputMode_GameAndUIEx` (`GameplayStatics.GetPlayerController` 0) null "LockAlways" false)
        (return true))
      (:`Is Not Valid`
        _)))
  (return false))

(fn `ShowHealthBar`
  (returns (WasSuccessful :type Boolean))
  (bind _returnvalue (`KismetSystemLibrary.K2_SetTimerDelegate` (`|CreateDelegate` :!event `UpdateHealthBarWidgetRotation`) (`self.HBRotationTickRate`) true))
  (set `self.HBRoationTickTimerRef` _returnvalue)
  (`SceneComponent.SetVisibility` (`self.HealthBar`) true false)
  (return true))

(fn `ShowSelectedIndicator`
  (returns (WasSuccessful :type Boolean))
  (bind _selectionindicatordecal (`self.SelectionIndicatorDecal`))
  (`ActorComponent.Activate` _selectionindicatordecal false)
  (`SceneComponent.SetVisibility` _selectionindicatordecal true false)
  (return true))

(fn `TakeDamage`
  (params (Damage :type "/Game/ASE/CombatLevel/DamageSystem/S_Damage Structure"))
  (returns (WasDamaged :type Boolean))
  (bind _damageapplied (`/Game/ASE/CombatLevel/DamageSystem/BPC_DamageSystem.TakeDamage` (`self.BPC_DamageSystem`) Damage))
  (return _damageapplied))

(fn `UpdateAllAbilitiesInfo`
  (params (UWB_AbilitiesBar :type "/Game/ASE/CombatLevel/UI/UWB_UnitAbilitiesBar Object Reference"))
  (bind _bpc_damagesystem (`self.BPC_DamageSystem`))
  (`|ExecutionSequence`
    (:`then_0`
      (`/Game/ASE/CombatLevel/UI/UWB_UnitAbilitiesBar.Update Attack` UWB_AbilitiesBar (`/Game/ASE/CombatLevel/DamageSystem/BPC_DamageSystem.Attack` _bpc_damagesystem)))
    (:`then_1`
      (`/Game/ASE/CombatLevel/UI/UWB_UnitAbilitiesBar.UpdateHealth` UWB_AbilitiesBar (`/Game/ASE/CombatLevel/DamageSystem/BPC_DamageSystem.Health` _bpc_damagesystem)))))

(fn `UserConstructionScript`
  (bind _bpc_damagesystem (`self.BPC_DamageSystem`))
  (`|ExecutionSequence`
    (:`then_0`
      (add `/Game/ASE/CombatLevel/DamageSystem/BPC_DamageSystem.OnDeath` _bpc_damagesystem (`|CreateDelegate` :!event `On Death`))
      (add `/Game/ASE/CombatLevel/DamageSystem/BPC_DamageSystem.OnBlocked` _bpc_damagesystem (`|CreateDelegate` :!event `On Damage Blocked`))
      (add `/Game/ASE/CombatLevel/DamageSystem/BPC_DamageSystem.OnDamageResponse` _bpc_damagesystem (`|CreateDelegate` :!event `On Damage Response`)))
    (:`then_1`
      (add `/Game/ASE/CombatLevel/DamageSystem/BPC_DamageSystem.OnHeathUpdated` _bpc_damagesystem (`|CreateDelegate` :!event `On Health Updated`))
      (add `/Game/ASE/CombatLevel/DamageSystem/BPC_DamageSystem.OnAttackUpdated` _bpc_damagesystem (`|CreateDelegate` :!event `On Attack Updated`)))))