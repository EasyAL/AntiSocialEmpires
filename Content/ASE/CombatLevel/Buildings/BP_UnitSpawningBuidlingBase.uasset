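; Base Blueprint for combat-level buildings that spawn units and answer selection-style calls such as faction, abilities and indicators.
; ShowAbilities creates a building abilities bar, binds its Unit A spawn event and sets game-and-UI input; HideAbilities removes it.
; SpawnGivenUnit calls an empty cost hook, then spawns the configured class at a random point in the spawn volume, adjusting for collisions.
; Health bar, selection indicator and movement functions are stubs returning false.
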(event `SpawnGivenUnit`
  (bind _spawningunitvolume (`self.SpawningUnitVolume`))
  (`self.SpawnUnitCost`)
  (bind _returnvalue (`|SpawnActorFromClass` (`self.UnitClassToSpawn`) (`KismetMathLibrary.Conv_VectorToTransform` (`KismetMathLibrary.RandomPointInBoundingBox` (`SceneComponent.K2_GetComponentLocation` _spawningunitvolume) (`BoxComponent.GetScaledBoxExtent` _spawningunitvolume))) "AdjustIfPossibleButDontSpawnIfColliding" "MultiplyWithRoot" null null))
  (`/Engine/EditorBlueprintResources/StandardMacros.IsValid` _returnvalue))

(fn `GetFaction`
  (returns (UnitsFaction :type "/Game/ASE/CombatLevel/CommandSystem/E_Faction Enum"))
  (return (`self.EFaction`)))

(fn `GetUnitType`
  (returns (IsBuilding :type Boolean))
  (return true))

(fn `HideAbilities`
  (returns (WasSuccessful :type Boolean))
  (bind _uwb_buildingcommandbarref (`self.UWB_BuildingCommandBarRef`))
  (`/Engine/EditorBlueprintResources/StandardMacros.IsValid` _uwb_buildingcommandbarref
    (:`Is Valid`
      (`Widget.RemoveFromParent` _uwb_buildingcommandbarref)
      (return true))
    (:`Is Not Valid`
      (return false))))

(fn `HideHealthBar`
  (returns (WasSuccessful :type Boolean))
  (return false))

(fn `HideSelectedIndicator`
  (returns (WasSuccessful :type Boolean))
  (return false))

(fn `MoveToLocation`
  (params (Destination :type "Vector Structure"))
  (returns (WasSuccessful :type Boolean))
  (return false))

(fn `ShowAbilities`
  (returns (WasSuccessful :type Boolean))
  (bind _returnvalue (`|CreateWidget` "/Game/ASE/CombatLevel/UI/UWB_BuildingAbilitiesBar.UWB_BuildingAbilitiesBar_C" (`GameplayStatics.GetPlayerController` 0)))
  (add `/Game/ASE/CombatLevel/UI/UWB_BuildingAbilitiesBar.SpawnUnitA` _returnvalue (`|CreateDelegate` :!event `SpawnGivenUnit`))
  (bind _output_get (set `self.UWB_BuildingCommandBarRef` _returnvalue))
  (`/Engine/EditorBlueprintResources/StandardMacros.IsValid` _output_get
    (:`Is Valid`
      (`UserWidget.AddToViewport` _returnvalue 0)
      (`WidgetBlueprintLibrary.SetInputMode_GameAndUIEx` (`GameplayStatics.GetPlayerController` 0) null "LockAlways" false)
      (return true))
    (:`Is Not Valid`
      (return false))))

(fn `ShowHealthBar`
  (returns (WasSuccessful :type Boolean))
  (return false))

(fn `ShowSelectedIndicator`
  (returns (WasSuccessful :type Boolean))
  (return false))

(fn `SpawnUnitCost`)

(fn `UserConstructionScript`)