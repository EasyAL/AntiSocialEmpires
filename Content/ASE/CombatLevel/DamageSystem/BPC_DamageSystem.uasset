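; BPC_DamageSystem is a component that manages an actor's health, healing, armour-mitigated damage and death.
; TakeDamage gates hits through CanBeDamaged, whose Block branch is unreachable because its outer check already sends blockable hits during blocking to No Damage.
; Armour gives diminishing-returns reduction via Armour / (Armour + 1500), after any percentage armour-ignore.
; ApplyDamage clamps health, then dispatches health-updated plus either death or damage-response events to listeners.
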(event `self.ReceiveBeginPlay`)

(fn `ApplyDamage`
  (params (DamageAmount :type "Float (double-precision)") (DamageResponse :type "/Game/ASE/CombatLevel/DamageSystem/E_DamageResponseType Enum" :default "NewEnumerator0"))
  ;[1 1 1] Deducting damage amount from health and check if we're dead and what response type we need to pass over to the owning actor
  (bind _output_get (set `self.Health` (`KismetMathLibrary.FClamp` (- (`self.Health`) DamageAmount) 0.0 (`self.MaxHealth`))))
  (`self.OnHeathUpdated`)
  (if (== _output_get 0.0)
    (set `self.IsDead` true)
    (`self.OnDeath`)
    (else
      (`self.OnDamageResponse` DamageResponse))))

(fn `ArmourDamageReduction`
  (params (Damage :type "Float (double-precision)") (IgnoreArmour :type "Float (double-precision)"))
  (returns (ReducedDamage :type "Float (double-precision)"))
  (bind _armour (`self.Armour`))
  ;[1 1 1] Reduce current armour by a percentage and then run it through my custom formula to get the new and reduced damage (DR% = Armour / (Armour + 1500))
  (if (== IgnoreArmour 0.0)
    (return (- Damage (* Damage (/ _armour (+ _armour 1500.0)))))
    (else
      (bind _reducedarmour (`self.ReduceArmour` (`self.Armour`) IgnoreArmour))
      (return (- Damage (* Damage (/ _reducedarmour (+ _reducedarmour 1500.0))))))))

(fn `Heal`
  (params (HealAmount :type "Float (double-precision)"))
  (returns (NewHealth :type "Float (double-precision)"))
  (if (not (`self.IsDead`))
    (bind _output_get (set `self.Health` (`KismetMathLibrary.FClamp` (+ HealAmount (`self.Health`)) 0.0 (`self.MaxHealth`))))
    (`self.OnHeathUpdated`)
    (return _output_get)))

(fn `ReduceArmour`
  (params (Armour :type "Float (double-precision)") (ReductionAmount :type "Float (double-precision)"))
  (returns (ReducedArmour :type "Float (double-precision)"))
  (return (`KismetMathLibrary.Conv_IntToDouble` (`KismetMathLibrary.Round` (- Armour (* Armour ReductionAmount))))))

(fn `TakeDamage`
  (params (IncomingDamage :type "/Game/ASE/CombatLevel/DamageSystem/S_Damage Structure"))
  (returns (DamageApplied :type Boolean))
  (`self.CanBeDamaged` IncomingDamage_IsUnblockableDamage_12_24F2B9A54E97B72F74C9FBB21B21879E
    (:`BlockDamage`
      (`self.OnBlocked`)
      (return false))
    (:`DealDamage`
      ;[1 1 1] Deal Damage Logic
      (bind _reduceddamage (`self.ArmourDamageReduction` IncomingDamage_DamageAmount_2_3239C4B14CB9BC11A540F682A2D7F166 IncomingDamage_IgnoreArmour_22_5D0644744214E2436659B1A6F8711997))
      (`self.ApplyDamage` _reduceddamage IncomingDamage_DamageResponse_8_6ADF217F4AFB4DC0DB3D078DBF2ED403)
      (return true))
    (:`NoDamage`
      (return false))))