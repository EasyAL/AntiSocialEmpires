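; BP_FirePit is a fire hazard that periodically deals armour-ignoring damage to BPI_Damageable actors inside its collision box.
; A looping timer starts when the first actor enters, damages the tracked overlapping actors and clears when the last one leaves.
; Through interface effect messages, entering grants a resistable attack buff and leaving applies a resistable burn-over-time debuff.
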(event `self.CollisionBox.OnComponentBeginOverlap`
  (params (OverlappedComponent :type "PrimitiveComponent Object Reference") (OtherActor :type "Actor Object Reference") (OtherComp :type "PrimitiveComponent Object Reference") (OtherBodyIndex :type Integer) (bFromSweep :type Boolean) (SweepResult :type "HitResult Structure (by ref)"))
  ;[1 1 1] If actor implements damageable interface, add them to the overlapping actors array and enable the timer by event function (if its not activated already) to continuously apply damage (also apply debuff once)
  (if (`KismetSystemLibrary.DoesImplementInterface` OtherActor "/Game/ASE/CombatLevel/DamageSystem/BPI_Damageable.BPI_Damageable_C")
    (`self.ActivateFireDamageEvent`)
    (`self.ApplyIncreaseAttackBuff` OtherActor)
    (`KismetArrayLibrary.Array_AddUnique` (`self.OverlappingActors`) OtherActor)))

(event `self.CollisionBox.OnComponentEndOverlap`
  (params (OverlappedComponent :type "PrimitiveComponent Object Reference") (OtherActor :type "Actor Object Reference") (OtherComp :type "PrimitiveComponent Object Reference") (OtherBodyIndex :type Integer))
  ;[1 1 1] Remove the actor from the array (if it implements damageable interface) and disable the timer by event function if the array is empty
  (if (`KismetSystemLibrary.DoesImplementInterface` OtherActor "/Game/ASE/CombatLevel/DamageSystem/BPI_Damageable.BPI_Damageable_C")
    (`KismetArrayLibrary.Array_RemoveItem` (`self.OverlappingActors`) OtherActor)
    (`self.DeactivateFireDamageEvent`)
    (`self.ApplyBurnOverTimeDebuff` OtherActor)))

(fn `ActivateFireDamageEvent`
  (bind _damagerate (`self.DamageRate`))
  (if (`KismetArrayLibrary.Array_IsEmpty` (`self.OverlappingActors`))
    (bind _returnvalue (`KismetSystemLibrary.K2_SetTimerDelegate` (`|CreateDelegate` :!event `Damage Overlapping Actors`) _damagerate true _damagerate))
    (set `self.EventTimerHandleRef` _returnvalue)))

(fn `ApplyBurnOverTimeDebuff`
  (params (Unit :type "Actor Object Reference"))
  (message `/Game/ASE/CombatLevel/EffectSystem/BPI_Effectable.ApplyEffect` Unit (make `/Game/ASE/CombatLevel/EffectSystem/S_Effect` "NewEnumerator4" 10.0 5.0 0.1 true 0.0 500.0)))

(fn `ApplyIncreaseAttackBuff`
  (params (Unit :type "Actor Object Reference"))
  (message `/Game/ASE/CombatLevel/EffectSystem/BPI_Effectable.ApplyEffect` Unit (make `/Game/ASE/CombatLevel/EffectSystem/S_Effect` "NewEnumerator1" 0.6 10.0 0.0 true 0.0 500.0)))

(fn `Damage Overlapping Actors`
  (for _array_element (`self.OverlappingActors`)
    (message `/Game/ASE/CombatLevel/DamageSystem/BPI_Damageable.TakeDamage` _array_element (make `/Game/ASE/CombatLevel/DamageSystem/S_Damage` 10.0 "NewEnumerator0" "NewEnumerator1" false false self 1.0))))

(fn `DeactivateFireDamageEvent`
  (if (`KismetArrayLibrary.Array_IsEmpty` (`self.OverlappingActors`))
    (`KismetSystemLibrary.K2_ClearAndInvalidateTimerHandle` (`self.EventTimerHandleRef`))))

(fn `UserConstructionScript`)