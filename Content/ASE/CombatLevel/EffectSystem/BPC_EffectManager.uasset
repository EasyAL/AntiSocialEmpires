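; Actor component that applies combat status effects to its owner, currently Increase Attack and Burn Over Time.
; ApplyEffect filters by immunity gameplay tags, then rolls resistable effects on caster accuracy minus Resistance.
; Successful effects spawn as BPC_Effect components, activate, join ActiveEffectsArray and return Applied.
; Only Increase Attack binds removal cleanup; Decrease Attack and Heal Over Time are unhandled and, like Increase Attack, check the DecreaseAttack immunity tag.
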(event `self.ReceiveBeginPlay`)

(fn `ApplyBurnOverTime`
  (params (Effect :type "/Game/ASE/CombatLevel/EffectSystem/S_Effect Structure"))
  (returns (Result :type "/Game/ASE/CombatLevel/EffectSystem/E_ApplyEffectResult Enum") (EffectRef :type "/Game/ASE/CombatLevel/EffectSystem/Effects/BPC_Effect_Base Object Reference"))
  (locals (LEffect :type "/Game/ASE/CombatLevel/EffectSystem/S_Effect Structure"))
  (bind ((`Severity_5_E93E6FA04F998750BBFBEBA3643A9B5C` _severity) (`Duration_7_E2BDECD94B034F05A0D5EC8D34005EDF` _duration) (`TickRate_9_5F5EE55A4874609D0A4DFB869BE31E40` _tickrate)) (break `/Game/ASE/CombatLevel/EffectSystem/S_Effect` (`local.LEffect`)))
  (bind _output_get (set `local.LEffect` Effect))
  (bind ((`Resistable_13_7B41DC29416AA9B0E7F73CAC217E93F4` _resistable) (`CastingActorsAccuracy_17_65D59F9F41A09803D44C0599D7AE8340` _castingactorsaccuracy)) (break `/Game/ASE/CombatLevel/EffectSystem/S_Effect` _output_get))
  (bind _applyeffect (`self.CheckIfEffectIsResisted` _resistable _castingactorsaccuracy))
  (if _applyeffect
    (bind _returnvalue (`|AddComponentByClass` (`self.GetOwner`) "/Game/ASE/CombatLevel/EffectSystem/Effects/BPC_Effect_OverTime_Burn.BPC_Effect_OverTime_Burn_C" _tickrate _severity _duration))
    (`/Game/ASE/CombatLevel/EffectSystem/Effects/BPC_Effect_Base.Activate Effect` _returnvalue)
    (`KismetArrayLibrary.Array_Add` (`self.ActiveEffectsArray`) _returnvalue)
    (return "NewEnumerator1" _returnvalue)
    (else
      (return "NewEnumerator2" null))))

(fn `ApplyEffect`
  (params (Effect :type "/Game/ASE/CombatLevel/EffectSystem/S_Effect Structure"))
  (returns (Result :type "/Game/ASE/CombatLevel/EffectSystem/E_ApplyEffectResult Enum") (EffectRef :type "/Game/ASE/CombatLevel/EffectSystem/Effects/BPC_Effect_Base Object Reference"))
  (locals (LEffect :type "/Game/ASE/CombatLevel/EffectSystem/S_Effect Structure"))
  (bind _leffect (`local.LEffect`))
  (bind _output_get (set `local.LEffect` Effect))
  (`self.AreWeImmune` _output_get
    (:`Non`
      (return "NewEnumerator0" null))
    (:`IncreaseAttack`
      (bind (_result _effectref) (`self.ApplyIncreaseAttack` _leffect))
      (`self.BindCleanupOnSuccessfulEffect` _result _effectref)
      (return _result _effectref))
    (:`BurnOverTime`
      (bind (_result_2 _effectref_2) (`self.ApplyBurnOverTime` _leffect))
      (return _result_2 _effectref_2))
    (:`Immune`
      (return "NewEnumerator3" null))))

(fn `ApplyIncreaseAttack`
  (params (Effect :type "/Game/ASE/CombatLevel/EffectSystem/S_Effect Structure"))
  (returns (Result :type "/Game/ASE/CombatLevel/EffectSystem/E_ApplyEffectResult Enum") (EffectRef :type "/Game/ASE/CombatLevel/EffectSystem/Effects/BPC_Effect_Base Object Reference"))
  (locals (LEffect :type "/Game/ASE/CombatLevel/EffectSystem/S_Effect Structure"))
  (bind ((`Severity_5_E93E6FA04F998750BBFBEBA3643A9B5C` _severity) (`Duration_7_E2BDECD94B034F05A0D5EC8D34005EDF` _duration)) (break `/Game/ASE/CombatLevel/EffectSystem/S_Effect` (`local.LEffect`)))
  (bind _output_get (set `local.LEffect` Effect))
  (bind ((`Resistable_13_7B41DC29416AA9B0E7F73CAC217E93F4` _resistable) (`CastingActorsAccuracy_17_65D59F9F41A09803D44C0599D7AE8340` _castingactorsaccuracy)) (break `/Game/ASE/CombatLevel/EffectSystem/S_Effect` _output_get))
  (bind _applyeffect (`self.CheckIfEffectIsResisted` _resistable _castingactorsaccuracy))
  (if _applyeffect
    (bind _returnvalue (`|AddComponentByClass` (`self.GetOwner`) "/Game/ASE/CombatLevel/EffectSystem/Effects/BPC_Effect_IncreaseAttack.BPC_Effect_IncreaseAttack_C" _severity _duration))
    (`/Game/ASE/CombatLevel/EffectSystem/Effects/BPC_Effect_Base.Activate Effect` _returnvalue)
    (`KismetArrayLibrary.Array_Add` (`self.ActiveEffectsArray`) _returnvalue)
    (return "NewEnumerator1" _returnvalue)
    (else
      (return "NewEnumerator2" null))))

(fn `BindCleanupOnSuccessfulEffect`
  (params (Result :type "/Game/ASE/CombatLevel/EffectSystem/E_ApplyEffectResult Enum" :default "NewEnumerator0") (EffectRef :type "/Game/ASE/CombatLevel/EffectSystem/Effects/BPC_Effect_Base Object Reference"))
  (switch `/Game/ASE/CombatLevel/EffectSystem/E_ApplyEffectResult` Result
    (:`NewEnumerator1`
      (add `/Game/ASE/CombatLevel/EffectSystem/Effects/BPC_Effect_Base.OnEffectRemoved` EffectRef (`|CreateDelegate` :!event `Remove Expired Effect`)))))

(fn `CheckIfEffectIsResisted`
  (params (Resistable :type Boolean) (CastingActorsAccuracy :type "Float (double-precision)"))
  (returns (ApplyEffect :type Boolean))
  (if Resistable
    (if (`KismetMathLibrary.RandomBoolWithWeight` (`KismetMathLibrary.MapRangeClamped` (- CastingActorsAccuracy (`self.Resistance`)) -100.0 100.0 0.0 1.0))
      (return true)
      (else
        (return false)))
    (else
      (return true))))

(fn `Remove Expired Effect`
  (params (EffectRef :type "/Game/ASE/CombatLevel/EffectSystem/Effects/BPC_Effect_Base Object Reference"))
  (bind _activeeffectsarray (`self.ActiveEffectsArray`))
  (bind _returnvalue (`Actor.K2_GetComponentsByClass` (`self.GetOwner` EffectRef) "/Game/ASE/CombatLevel/EffectSystem/Effects/BPC_Effect_Base.BPC_Effect_Base_C"))
  (`KismetArrayLibrary.Array_Remove` _activeeffectsarray (`KismetArrayLibrary.Array_Find` _activeeffectsarray EffectRef))
  (`self.K2_DestroyComponent` (`|GetArrayItem` _returnvalue (`KismetArrayLibrary.Array_Find` _returnvalue EffectRef))))