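; Effect component in the combat effect system that temporarily raises the owner's Attack stat.
; Activation adds MaxAttack scaled by Severity to Attack on the referenced damage system component and starts a one-shot timer for Duration.
; Deactivation subtracts the same formula, recomputed from current values rather than a stored bonus, then calls the parent deactivation.
; Both paths notify the damage system that Attack has changed.
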(event `self.Activate Effect`
  (bind _damagesystemcomponentref (`self.DamageSystemComponentRef`))
  (set `/Game/ASE/CombatLevel/DamageSystem/BPC_DamageSystem.Attack` (+ (* (`/Game/ASE/CombatLevel/DamageSystem/BPC_DamageSystem.MaxAttack` _damagesystemcomponentref) (`self.Severity`)) (`/Game/ASE/CombatLevel/DamageSystem/BPC_DamageSystem.Attack` _damagesystemcomponentref)) _damagesystemcomponentref)
  (`KismetSystemLibrary.K2_SetTimerDelegate` (`|CreateDelegate` :!event `Deactivate Effect`) (`self.Duration`))
  (`/Game/ASE/CombatLevel/DamageSystem/BPC_DamageSystem.OnAttackUpdated` _damagesystemcomponentref))

(event `self.Deactivate Effect`
  (bind _damagesystemcomponentref (`self.DamageSystemComponentRef`))
  (set `/Game/ASE/CombatLevel/DamageSystem/BPC_DamageSystem.Attack` (- (`/Game/ASE/CombatLevel/DamageSystem/BPC_DamageSystem.Attack` _damagesystemcomponentref) (* (`/Game/ASE/CombatLevel/DamageSystem/BPC_DamageSystem.MaxAttack` _damagesystemcomponentref) (`self.Severity`))) _damagesystemcomponentref)
  (`/Game/ASE/CombatLevel/DamageSystem/BPC_DamageSystem.OnAttackUpdated` _damagesystemcomponentref)
  (`parent.Deactivate Effect`))