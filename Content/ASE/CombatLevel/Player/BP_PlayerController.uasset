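; Player controller for the combat level that handles camera movement, look, zoom and RTS-style unit selection and commands via Enhanced Input.
; Toggle or hold inputs switch between free look and a cursor mode, which gates selection input.
; Clicks select or move units through a visibility trace, interface messages and faction checks, while drags take box selections from the HUD.
; Enemy targeting is only a print stub.
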(event `self.ReceiveBeginPlay`
  (bind _returnvalue (subsystem `EnhancedInputLocalPlayerSubsystem`))
  ;[1 1 1] IMC setup
  (`/Engine/EditorBlueprintResources/StandardMacros.IsValid` _returnvalue
    (:`Is Valid`
      (`EnhancedInputSubsystemInterface.AddMappingContext` _returnvalue "/Game/ASE/CombatLevel/Player/Input/IMC_Combat.IMC_Combat" 0 (struct)))))

(event `EnhancedInput|/Game/ASE/CombatLevel/Player/Input/IA_Look`
  (params (ActionValue :type "Vector2D Structure") (ElapsedSeconds :type "Float (double-precision)") (TriggeredSeconds :type "Float (double-precision)") (InputAction :type "InputAction Object Reference" :default "/Game/ASE/CombatLevel/Player/Input/IA_Look.IA_Look"))
  ;[1 1 1] Camera Look Around Input Handling
  (:`Triggered`
    (`self.AddYawInput` ActionValue_X)
    (`self.AddPitchInput` ActionValue_Y)))

(event `EnhancedInput|/Game/ASE/CombatLevel/Player/Input/IA_MoveH`
  (params (ActionValue :type "Vector2D Structure") (ElapsedSeconds :type "Float (double-precision)") (TriggeredSeconds :type "Float (double-precision)") (InputAction :type "InputAction Object Reference" :default "/Game/ASE/CombatLevel/Player/Input/IA_MoveH.IA_MoveH"))
  (bind _returnvalue (`self.K2_GetPawn`))
  (bind (_returnvalue_roll _returnvalue_pitch _returnvalue_yaw) (`KismetMathLibrary.BreakRotator` (`self.GetControlRotation`)))
  ;[1 1 1] Movement Input Handling
  (:`Triggered`
    (`Pawn.AddMovementInput` _returnvalue (`KismetMathLibrary.GetRightVector` (`KismetMathLibrary.MakeRotator` _returnvalue_roll 0.0 _returnvalue_yaw)) ActionValue_X false)
    (`Pawn.AddMovementInput` _returnvalue (`KismetMathLibrary.GetForwardVector` (`KismetMathLibrary.MakeRotator` 0.0 0.0 _returnvalue_yaw)) ActionValue_Y false)))

(event `EnhancedInput|/Game/ASE/CombatLevel/Player/Input/IA_ClearUnitSelection`
  (params (ActionValue :type Boolean) (ElapsedSeconds :type "Float (double-precision)") (TriggeredSeconds :type "Float (double-precision)") (InputAction :type "InputAction Object Reference" :default "/Game/ASE/CombatLevel/Player/Input/IA_ClearUnitSelection.IA_ClearUnitSelection"))
  ;[1 1 1] Deselects all units and clears all containers
  (:`Started`
    (`|ExecutionSequence`
      (:`then_0`
        (`self.DeselectGivenUnit` (`self.SelectedUnit`) true))
      (:`then_1`
        (`self.DeselectArrayOfUnits` (`self.SelectionOfUnits`) true)))))

(event `EnhancedInput|/Game/ASE/CombatLevel/Player/Input/IA_CursorLookToggle`
  (params (ActionValue :type Boolean) (ElapsedSeconds :type "Float (double-precision)") (TriggeredSeconds :type "Float (double-precision)") (InputAction :type "InputAction Object Reference" :default "/Game/ASE/CombatLevel/Player/Input/IA_CursorLookToggle.IA_CursorLookToggle"))
  ;[1 1 1] Cursor Pointing Mode Handling (Toggle between cursor pointing and free look by clicking RMB)
  (:`Started`
    (`self.KitKat`
      (:`execA`
        (set `self.bShowMouseCursor` true) ; On Clicked, show cursor and ignore look
        (`WidgetBlueprintLibrary.SetInputMode_GameAndUIEx` self null "LockAlways" false)
        (`self.SetIgnoreLookInput` true)
        (`self.SetMouseCursorPositionToMiddleOfScreen`))
      (:`execB`
        (set `self.bShowMouseCursor` false) ; On released, hide cursor and set game only mode
        (`WidgetBlueprintLibrary.SetInputMode_GameOnly` self)
        (`self.SetIgnoreLookInput` false)))))

(event `EnhancedInput|/Game/ASE/CombatLevel/Player/Input/IA_CursorLookHold`
  (params (ActionValue :type Boolean) (ElapsedSeconds :type "Float (double-precision)") (TriggeredSeconds :type "Float (double-precision)") (InputAction :type "InputAction Object Reference" :default "/Game/ASE/CombatLevel/Player/Input/IA_CursorLookHold.IA_CursorLookHold"))
  ;[1 1 1] Cursor Pointing Mode Handling (switch between cursor pointing and free look while holding Shift)
  (:`Started`
    (if (`self.KitKatSwitchBool`)
      (set `self.KitKatSwitchBool` false)
      (set `self.bShowMouseCursor` true) ; On Clicked, show cursor and ignore look
      (`WidgetBlueprintLibrary.SetInputMode_GameAndUIEx` self null "LockAlways" false)
      (`self.SetIgnoreLookInput` true)
      (`self.SetMouseCursorPositionToMiddleOfScreen`)))
  (:`Completed`
    (if (not (`self.KitKatSwitchBool`))
      (set `self.KitKatSwitchBool` true)
      (set `self.bShowMouseCursor` false) ; On released, hide cursor and set game only mode
      (`WidgetBlueprintLibrary.SetInputMode_GameOnly` self)
      (`self.SetIgnoreLookInput` false))))

(event `EnhancedInput|/Game/ASE/CombatLevel/Player/Input/IA_Select`
  (params (ActionValue :type Boolean) (ElapsedSeconds :type "Float (double-precision)") (TriggeredSeconds :type "Float (double-precision)") (InputAction :type "InputAction Object Reference" :default "/Game/ASE/CombatLevel/Player/Input/IA_Select.IA_Select"))
  (bind _returnvalue (`self.GetHUD`))
  ;[1 1 1] On Click, Perform line trace under mouse cursor and show the debug line
  (:`Triggered`
    (`self.WhenMouseCursorShowing` (`self.bShowMouseCursor`) :!label _label
      (:`Output One`
        (message `/Game/ASE/CombatLevel/UI/BPI_HUDAndControllerCommunication.SelectionTick` _returnvalue) ; Called over and over once delay is overcome
      )
      (:`Output Two`
        (message `/Game/ASE/CombatLevel/UI/BPI_HUDAndControllerCommunication.SelectionInit` _returnvalue) ; Called on click,
      )
      (:`Output Three`
        (if (`KismetArrayLibrary.Array_IsNotEmpty` (`self.SelectionOfUnits`))
          (`self.HandleSelectionOfUnitsActionsBasedOnContext`) ; Direct behaviour of all units in the selection based on what we click
          (else
            (`/Engine/EditorBlueprintResources/StandardMacros.IsValid` (`self.SelectedUnit`) ; If array is empty and cached unit is not
              (:`Is Valid`
                (`self.HandleUnitsActionsBasedOnContext`) ; Direct behaviour of cached unit based on what we click
              )
              (:`Is Not Valid`
                (`self.SelectUnit`) ; Both containers are empty hence, try and save unit under cursor
              )))))
      (:`Output Four`
        (message `/Game/ASE/CombatLevel/UI/BPI_HUDAndControllerCommunication.SelectionEnd` _returnvalue) ; Called on releasing click
        (bind _selectedunits (message `/Game/ASE/CombatLevel/UI/BPI_HUDAndControllerCommunication.GetSelectedUnits` _returnvalue))
        (bind _output_get (set `self.SelectionOfUnits` _selectedunits))
        ;;[0 0 0] See if select unit is within 'selection of units'. If true, we hide its abilities bar and clear selected unit bar, else we deselect it.
        (if (!= (`KismetArrayLibrary.Array_Find` _output_get (`self.SelectedUnit`)) -1)
          (`self.DeselectUnitByBools` (`self.SelectedUnit`) true)
          (set `self.SelectedUnit` null)
          (else
            (`self.DeselectGivenUnit` (`self.SelectedUnit`) true))))))
  (:`Started`
    (goto _label :!via `Exec Two`))
  (:`Canceled`
    (goto _label :!via `Exec Three`))
  (:`Completed`
    (goto _label :!via `Exec Four`)))

(event `EnhancedInput|/Game/ASE/CombatLevel/Player/Input/IA_Zoom`
  (params (ActionValue :type "Float (double-precision)") (ElapsedSeconds :type "Float (double-precision)") (TriggeredSeconds :type "Float (double-precision)") (InputAction :type "InputAction Object Reference" :default "/Game/ASE/CombatLevel/Player/Input/IA_Zoom.IA_Zoom"))
  (bind (_returnvalue_roll _returnvalue_pitch _returnvalue_yaw) (`KismetMathLibrary.BreakRotator` (`self.GetControlRotation`)))
  ;[1 1 1] Needs Work
  (:`Triggered`
    (message `/Game/ASE/CombatLevel/Player/BPI_CameraMovement.AddMovement` (`self.K2_GetPawn`) (`KismetMathLibrary.GetForwardVector` (`KismetMathLibrary.MakeRotator` _returnvalue_roll _returnvalue_pitch _returnvalue_yaw)) 1250.0 ActionValue)))

(fn `ActiveCursorMode`
  (bind _returnvalue (`GameplayStatics.GetPlayerController` 0))
  (set `self.bShowMouseCursor` true) ; On Clicked, show cursor and ignore look
  (`WidgetBlueprintLibrary.SetInputMode_GameAndUIEx` _returnvalue null "LockAlways" false)
  (`self.SetIgnoreLookInput` _returnvalue true)
  (`self.SetMouseCursorPositionToMiddleOfScreen`))

(fn `CheckForCommandableActorUnderMouse`
  (returns (IsCommandable :type Boolean) (HitActor :type "Actor Object Reference") (HitLocation :type "Vector Structure"))
  (bind (_bblockinghit _binitialoverlap _time _distance _location _impactpoint _normal _impactnormal _physmat _hitactor) (`GameplayStatics.BreakHitResult` (`self.GetHitResultUnderCursorByChannel` "TraceTypeQuery1")))
  (if (`KismetSystemLibrary.DoesImplementInterface` _hitactor "/Game/ASE/CombatLevel/CommandSystem/BPI_Commandable.BPI_Commandable_C")
    (return true _hitactor _location)
    (else
      (return false null _location))))

(fn `DeselectArrayOfUnits`
  (params (Units :type "Array of Actor Object Reference") (ClearArray :type Boolean))
  ;[1 1 1] Deselects array of units one by one and then clears the array if upon request
  (if (`KismetArrayLibrary.Array_IsNotEmpty` Units)
    (for _array_element Units
      (`self.DeselectionTasksByFaction` _array_element))
    (if ClearArray
      (`KismetArrayLibrary.Array_Clear` Units))))

(fn `DeselectGivenUnit`
  (params (Unit :type "Actor Object Reference") (`Clear Ref` :type Boolean))
  ;[1 1 1] Deselects passed unit and clears the ref variable upon request
  (`/Engine/EditorBlueprintResources/StandardMacros.IsValid` Unit
    (:`Is Valid`
      (`self.DeselectionTasksByFaction` Unit)
      (if `Clear Ref`
        (set `self.SelectedUnit` null)))))

(fn `DeselectionTasksByFaction`
  (params (Actor :type "Actor Object Reference"))
  (bind _unitsfaction (message `/Game/ASE/CombatLevel/CommandSystem/BPI_Commandable.GetFaction` Actor))
  (switch `/Game/ASE/CombatLevel/CommandSystem/E_Faction` _unitsfaction
    (:`NewEnumerator6`
      (`KismetSystemLibrary.PrintString` "We do nothing" false))
    (:`NewEnumerator7`
      (`KismetSystemLibrary.PrintString` "We deselected friendly Unit!" false)
      (message `/Game/ASE/CombatLevel/CommandSystem/BPI_Commandable.HideHealthBar` Actor :!label _label)
      (message `/Game/ASE/CombatLevel/CommandSystem/BPI_Commandable.HideSelectedIndicator` Actor)
      (message `/Game/ASE/CombatLevel/CommandSystem/BPI_Commandable.HideAbilities` Actor))
    (:`NewEnumerator8`
      (`KismetSystemLibrary.PrintString` "We deselected Allied Unit!" false)
      (goto _label))
    (:`NewEnumerator9`
      (`KismetSystemLibrary.PrintString` "We deselected neutral Unit!" false)
      (goto _label))
    (:`NewEnumerator10`
      (`KismetSystemLibrary.PrintString` "We deselected enemy Unit!" false)
      (message `/Game/ASE/CombatLevel/CommandSystem/BPI_Commandable.HideHealthBar` Actor)
      (message `/Game/ASE/CombatLevel/CommandSystem/BPI_Commandable.HideSelectedIndicator` Actor))
    (:`NewEnumerator11`
      (`KismetSystemLibrary.PrintString` "We deselected exposed enemy Unit!" false)
      (goto _label))))

(fn `DeselectUnitByBools`
  (params (Unit :type "Actor Object Reference") (HideSkillBar :type Boolean) (HideHealthBar :type Boolean) (HideSelectedIndicator :type Boolean))
  (locals (LUnit :type "Actor Object Reference"))
  (`/Engine/EditorBlueprintResources/StandardMacros.IsValid` Unit
    (:`Is Valid`
      (set `local.LUnit` Unit)
      (`|ExecutionSequence`
        (:`then_0`
          (if HideSkillBar
            (message `/Game/ASE/CombatLevel/CommandSystem/BPI_Commandable.HideAbilities` (`local.LUnit`))))
        (:`then_1`
          (if HideHealthBar
            (message `/Game/ASE/CombatLevel/CommandSystem/BPI_Commandable.HideHealthBar` (`local.LUnit`))))
        (:`then_2`
          (if HideSelectedIndicator
            (message `/Game/ASE/CombatLevel/CommandSystem/BPI_Commandable.HideSelectedIndicator` (`local.LUnit`))))))))

(fn `HandleSelectedUnitsActionsByTargetsFaction`
  (params (HitActor :type "Actor Object Reference"))
  (bind _unitsfaction (message `/Game/ASE/CombatLevel/CommandSystem/BPI_Commandable.GetFaction` HitActor))
  (switch `/Game/ASE/CombatLevel/CommandSystem/E_Faction` _unitsfaction
    (:`NewEnumerator6`
      (`KismetSystemLibrary.PrintString` "We do nothing"))
    (:`NewEnumerator7`
      (`self.DeselectArrayOfUnits` (`self.SelectionOfUnits`) true :!label _label)
      (`self.SelectionTasksByFaction` HitActor)
      (set `self.SelectedUnit` HitActor))
    (:`NewEnumerator8`
      (goto _label))
    (:`NewEnumerator10`
      (`KismetSystemLibrary.PrintString` "We will give enemy location to our unit!" :!label _label_2))
    (:`NewEnumerator11`
      (goto _label_2))))

(fn `HandleSelectionOfUnitsActionsBasedOnContext`
  (bind (_iscommandable _hitactor _hitlocation) (`self.CheckForCommandableActorUnderMouse`))
  (if _iscommandable
    (`self.HandleSelectedUnitsActionsByTargetsFaction` _hitactor)
    (else
      (`self.MoveSelectionOfUnits` (`self.SelectionOfUnits`) _hitlocation))))

(fn `HandleUnitActionByTargetsFaction`
  (params (HitActor :type "Actor Object Reference"))
  (bind _unitsfaction (message `/Game/ASE/CombatLevel/CommandSystem/BPI_Commandable.GetFaction` HitActor))
  (switch `/Game/ASE/CombatLevel/CommandSystem/E_Faction` _unitsfaction
    (:`NewEnumerator6`
      (`KismetSystemLibrary.PrintString` "We do nothing"))
    (:`NewEnumerator7`
      (`self.DeselectionTasksByFaction` (`self.SelectedUnit`) :!label _label)
      (set `self.SelectedUnit` null)
      (`self.SelectionTasksByFaction` HitActor)
      (set `self.SelectedUnit` HitActor))
    (:`NewEnumerator8`
      (goto _label))
    (:`NewEnumerator10`
      (`KismetSystemLibrary.PrintString` "We will give enemy location to our unit!" :!label _label_2))
    (:`NewEnumerator11`
      (goto _label_2))))

(fn `HandleUnitsActionsBasedOnContext`
  (bind _selectedunit (`self.SelectedUnit`))
  (bind _isbuilding (message `/Game/ASE/CombatLevel/CommandSystem/BPI_Commandable.GetUnitType` _selectedunit))
  (if (not _isbuilding)
    (bind (_iscommandable _hitactor _hitlocation) (`self.CheckForCommandableActorUnderMouse`))
    (if _iscommandable
      (`self.HandleUnitActionByTargetsFaction` _hitactor)
      (else
        (`self.MoveSingleUnit` (`self.SelectedUnit`) _hitlocation)))
    (else
      ;[1 1 1] If building, deselect on clicking anything and check if we can select a unit under cursor
      (`self.DeselectionTasksByFaction` _selectedunit)
      (set `self.SelectedUnit` null)
      (bind (_iscommandable_2 _hitactor_2) (`self.CheckForCommandableActorUnderMouse`))
      (if _iscommandable_2
        (bind _unitsfaction (message `/Game/ASE/CombatLevel/CommandSystem/BPI_Commandable.GetFaction` _hitactor_2))
        (switch `/Game/ASE/CombatLevel/CommandSystem/E_Faction` _unitsfaction
          (:`NewEnumerator7`
            _)
          (:`NewEnumerator8`
            _))
        (`self.SelectionTasksByFaction` _hitactor_2)
        (set `self.SelectedUnit` _hitactor_2)))))

(fn `InactiveCursorMode`
  (bind _returnvalue (`GameplayStatics.GetPlayerController` 0))
  ;[1 1 1] Successful Release
  (set `self.bShowMouseCursor` false) ; On released, hide cursor and set game only mode
  (`WidgetBlueprintLibrary.SetInputMode_GameOnly` _returnvalue true)
  (`self.SetIgnoreLookInput` _returnvalue false))

(fn `MoveSelectionOfUnits`
  (params (Units :type "Array of Actor Object Reference") (TargetLocation :type "Vector Structure"))
  (for _array_element Units
    (bind _wassuccessful (message `/Game/ASE/CombatLevel/CommandSystem/BPI_Commandable.MoveToLocation` _array_element TargetLocation)))
  (if _wassuccessful
    (`NiagaraFunctionLibrary.SpawnSystemAtLocation` "/Game/Cursor/FX_Cursor.FX_Cursor")))

(fn `MoveSingleUnit`
  (params (Unit :type "Actor Object Reference") (TargetLocation :type "Vector Structure"))
  (bind _wassuccessful (message `/Game/ASE/CombatLevel/CommandSystem/BPI_Commandable.MoveToLocation` Unit TargetLocation))
  (if _wassuccessful
    (`NiagaraFunctionLibrary.SpawnSystemAtLocation` "/Game/Cursor/FX_Cursor.FX_Cursor")))

(fn `SelectionTasksByFaction`
  (params (Actor :type "Actor Object Reference"))
  (bind _unitsfaction (message `/Game/ASE/CombatLevel/CommandSystem/BPI_Commandable.GetFaction` Actor))
  (switch `/Game/ASE/CombatLevel/CommandSystem/E_Faction` _unitsfaction
    (:`NewEnumerator6`
      (`KismetSystemLibrary.PrintString` "We do nothing" false))
    (:`NewEnumerator7`
      (`KismetSystemLibrary.PrintString` "We selected friendly Unit!" false)
      (message `/Game/ASE/CombatLevel/CommandSystem/BPI_Commandable.ShowHealthBar` Actor :!label _label)
      (message `/Game/ASE/CombatLevel/CommandSystem/BPI_Commandable.ShowSelectedIndicator` Actor)
      (message `/Game/ASE/CombatLevel/CommandSystem/BPI_Commandable.ShowAbilities` Actor))
    (:`NewEnumerator8`
      (`KismetSystemLibrary.PrintString` "We selected Allied Unit!" false)
      (goto _label))
    (:`NewEnumerator9`
      (`KismetSystemLibrary.PrintString` "We selected neutral Unit!" false)
      (goto _label))
    (:`NewEnumerator10`
      (`KismetSystemLibrary.PrintString` "We selected enemy Unit!" false)
      (message `/Game/ASE/CombatLevel/CommandSystem/BPI_Commandable.ShowHealthBar` Actor)
      (message `/Game/ASE/CombatLevel/CommandSystem/BPI_Commandable.ShowSelectedIndicator` Actor))
    (:`NewEnumerator11`
      (`KismetSystemLibrary.PrintString` "We selected exposed enemy Unit!" false)
      (goto _label))))

(fn `SelectUnit`
  (bind (_iscommandable _hitactor) (`self.CheckForCommandableActorUnderMouse`))
  (if _iscommandable
    (`self.SelectionTasksByFaction` _hitactor)
    (set `self.SelectedUnit` _hitactor)))

(fn `SetMouseCursorPositionToMiddleOfScreen`
  (bind (_returnvalue_x _returnvalue_y) (`KismetMathLibrary.BreakVector2D` (* (`WidgetLayoutLibrary.GetViewportSize`) (0.5 0.5))))
  ;[1 1 1] Sets the position of the mouse cursor to the center of the screen
  (`self.SetMouseLocation` (`KismetMathLibrary.FTrunc` _returnvalue_x) (`KismetMathLibrary.FTrunc` _returnvalue_y)))

(fn `UserConstructionScript`)