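; Combat damage component that tracks an actor's health and death, with early scaffolding for buffs and debuffs.
; TakeDamage gates hits through CanBeDamaged, reduces them with a diminishing-returns armour formula supporting partial armour ignore, then fires death or damage-response dispatchers.
; Heal returns clamped health without storing it, and CanBeDamaged's block branch is unreachable.
; Debuffs roll accuracy against resistance but only print, while ReceiveBuff and the debuff-array loop are empty.
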(event `self.ReceiveBeginPlay`
  (`KismetSystemLibrary.K2_SetTimerDelegate` (`|CreateDelegate` :!event `Manage Buff And Debuff System`) 1.0 true))

(event `Manage Buff And Debuff System`
  (for _ (`self.DebuffArray`)
    _))

(fn `ApplyDamage`
  (params (DamageAmount :type "Float (double-precision)") (DamageResponse :type "/Game/Base/CombatLevel/DamageSystem/E_DamageResponseType Enum" :default "NewEnumerator0"))
  ;[1 1 1] Deducting damage amount from health and check if we're dead and what response type we need to pass over to the owning actor
  (bind _output_get (set `self.Health` (`KismetMathLibrary.FClamp` (- (`self.Health`) DamageAmount) 0.0 (`self.MaxHealth`))))
  (if (== _output_get 0.0)
    (set `self.IsDead` true)
    (`self.OnDeath`)
    (else
      (`self.OnDamageResponse` DamageResponse))))

(fn `ArmourDamageReduction`
  (params (Damage :type "Float (double-precision)") (IgnoreArmour :type "Float (double-precision)"))
  (returns (ReducedDamage :type "Float (double-precision)"))
  (bind _armour (`self.Armour`))
  ;[1 1 1] Reduce current armour by a percentage and then run it through my custom formula to get the new and reduced damage (DR% = Armour / (Armour + 1500))
  (if (== IgnoreArmour 0.0)
    (return (- Damage (* Damage (/ _armour (+ _armour 1500.0)))))
    (else
      (bind _reducedarmour (`self.ReduceArmour` (`self.Armour`) IgnoreArmour))
      (return (- Damage (* Damage (/ _reducedarmour (+ _reducedarmour 1500.0))))))))

(fn `Heal`
  (params (HealAmount :type "Float (double-precision)"))
  (returns (NewHealth :type "Float (double-precision)"))
  (if (not (`self.IsDead`))
    (return (`KismetMathLibrary.FClamp` (+ HealAmount (`self.Health`)) 0.0 (`self.MaxHealth`)))))

(fn `ReceiveBuff`)

(fn `ReceiveDebuff`
  (params (Debuff :type "/Game/Base/CombatLevel/DamageSystem/S_Debuff Structure"))
  (returns (DebuffApplied :type Boolean))
  (locals (LDebuff :type "/Game/Base/CombatLevel/DamageSystem/E_Debuff Enum"))
  (bind (_debuff _duration _severity _timeofapplication _castingactorsaccuracy _castingactor _canberesisted) (break `/Game/Base/CombatLevel/DamageSystem/S_Debuff` Debuff))
  (if _canberesisted
    (if (`KismetMathLibrary.RandomBoolWithWeight` (/ _castingactorsaccuracy (`self.Resistance`)))
      ;[1 1 1] Check which debuff it is
      (switch `/Game/Base/CombatLevel/DamageSystem/E_Debuff` _debuff :!label _label
        (:`NewEnumerator0`
          _)
        (:`NewEnumerator1`
          (`KismetSystemLibrary.PrintString` (`|GetEnumeratorNameAsString` _debuff))
          (return true))))
    (else
      (goto _label)))
  ;[1 1 1] Actor Resisted the Debuff
  (return false))

(fn `ReduceArmour`
  (params (Armour :type "Float (double-precision)") (ReductionAmount :type "Float (double-precision)"))
  (returns (ReducedArmour :type "Float (double-precision)"))
  (return (`KismetMathLibrary.Conv_IntToDouble` (`KismetMathLibrary.Round` (- Armour (* Armour ReductionAmount))))))

(fn `TakeDamage`
  (params (IncomingDamage :type "/Game/Base/CombatLevel/DamageSystem/S_Damage Structure"))
  (returns (DamageApplied :type Boolean))
  (`self.CanBeDamaged` IncomingDamage_IsUnblockableDamage_12_24F2B9A54E97B72F74C9FBB21B21879E
    (:`BlockDamage`
      (`self.OnBlocked`)
      (return false))
    (:`DealDamage`
      ;[1 1 1] Deal Damage Logic
      (bind _reduceddamage (`self.ArmourDamageReduction` IncomingDamage_DamageAmount_2_3239C4B14CB9BC11A540F682A2D7F166 IncomingDamage_IgnoreArmour_22_5D0644744214E2436659B1A6F8711997))
      (`self.ApplyDamage` _reduceddamage IncomingDamage_DamageResponse_8_6ADF217F4AFB4DC0DB3D078DBF2ED403)
      (return true))
    (:`NoDamage`
      (`KismetSystemLibrary.PrintString` "No Damage Applied!")
      (return false))))