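; BP_FirePit is a hazard actor that periodically damages and debuffs an actor inside its collision box.
; A looping one-second timer, started on BeginPlay, sends armour-ignoring damage and a resistible debuff through message calls.
; Overlap events track a single OtherActor, so a new entrant replaces the previous target and any exit clears it.
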(event `self.ReceiveBeginPlay`
  (`KismetSystemLibrary.K2_SetTimerDelegate` (delegate `Damage Overlapping Actor`) 1.0 true 1.0))

(event `Damage Overlapping Actor`
  (bind _other_actor (`self.Other Actor`))
  (`/Engine/EditorBlueprintResources/StandardMacros.IsValid` _other_actor
    (:`Is Valid`
      (message `/Game/Base/CombatLevel/DamageSystem/BPI_Damageable.TakeDamage` _other_actor (make `/Game/Base/CombatLevel/DamageSystem/S_Damage` 25.0 "NewEnumerator0" "NewEnumerator1" false false self 1.0))
      (message `/Game/Base/CombatLevel/DamageSystem/BPI_Damageable.ApplyDebuff` _other_actor (make `/Game/Base/CombatLevel/DamageSystem/S_Debuff` "NewEnumerator1" 15.0 0.5 0.0 100.0 self true)))))

(event `self.CollisionBox.OnComponentBeginOverlap`
  (params (OverlappedComponent :type "PrimitiveComponent Object Reference") (OtherActor :type "Actor Object Reference") (OtherComp :type "PrimitiveComponent Object Reference") (OtherBodyIndex :type Integer) (bFromSweep :type Boolean) (SweepResult :type "HitResult Structure (by ref)"))
  (set `self.Other Actor` OtherActor))

(event `self.CollisionBox.OnComponentEndOverlap`
  (params (OverlappedComponent :type "PrimitiveComponent Object Reference") (OtherActor :type "Actor Object Reference") (OtherComp :type "PrimitiveComponent Object Reference") (OtherBodyIndex :type Integer))
  (set `self.Other Actor` null))

(fn `UserConstructionScript`)