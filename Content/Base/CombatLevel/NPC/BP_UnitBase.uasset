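; Base combat unit character that can be selected, moved, damaged, healed and debuffed, with buffs left as a stub.
; BPCDamageSystem owns health and death events, while the unit updates its health bar and shows or hides its ability bar and selection indicator.
; A looping timer, active while the health bar shows, turns it toward the camera.
; Death ragdolls the mesh, then randomly destroys the actor or revives it at full health using the cached mesh transform.
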(event `self.ReceiveBeginPlay`
  (`self.InitHealthBar`))

(event `On Death`
  (bind _mesh (`self.Mesh`))
  ;[1 1 1] Saves the meshes transform incase of revive... then enables ragdol and collision, hides some UI elements before going into a 5 sec wait... in the end, a 50% chance of death vs revive
  (`CharacterMovementComponent.DisableMovement` (`self.CharacterMovement`))
  (set `self.MeshTransformCache` (`SceneComponent.K2_GetComponentToWorld` (`self.Mesh`)))
  (`PrimitiveComponent.SetSimulatePhysics` _mesh true)
  (`PrimitiveComponent.SetCollisionEnabled` _mesh "QueryAndPhysics")
  (`/Game/Base/CombatLevel/CommandSystem/BPI_Commandable.HideHealthBar`)
  (`/Game/Base/CombatLevel/CommandSystem/BPI_Commandable.HideAbilities`)
  (`/Game/Base/CombatLevel/CommandSystem/BPI_Commandable.HideSelectedIndicator`)
  (`KismetSystemLibrary.Delay` 5.0)
  (if (`KismetMathLibrary.RandomBool`)
    (`self.K2_DestroyActor`)
    (else
      (`self.On Revive`))))

(event `On Revive`
  (bind _bpc_damagesystem (`self.BPC_DamageSystem`))
  (bind _mesh (`self.Mesh`))
  ;[1 1 1] Revives Actor with 100% HP
  (`PrimitiveComponent.SetSimulatePhysics` _mesh false)
  (`PrimitiveComponent.SetCollisionEnabled` _mesh "NoCollision")
  (`SceneComponent.K2_SetWorldTransform` _mesh (`self.MeshTransformCache`) true false)
  (`CharacterMovementComponent.SetMovementMode` (`self.CharacterMovement`) "MOVE_Walking" 0)
  (set `/Game/Base/CombatLevel/DamageSystem/BPC_DamageSystem.IsDead` false _bpc_damagesystem)
  (`self.Heal` (`/Game/Base/CombatLevel/DamageSystem/BPC_DamageSystem.MaxHealth` _bpc_damagesystem)))

(event `UpdateHealthBarWidgetRotation`
  (bind _healthbar (`self.HealthBar`))
  ;[1 1 1] Ensures actors health bar is always facing camera
  (`SceneComponent.K2_SetWorldRotation` _healthbar (`KismetMathLibrary.FindLookAtRotation` (`SceneComponent.K2_GetComponentLocation` _healthbar) (`SceneComponent.K2_GetComponentLocation` (`PlayerCameraManager.TransformComponent` (`GameplayStatics.GetPlayerCameraManager` 0)))) false false))

(event `On Damage Response`
  (params (ResponseType :type "/Game/Base/CombatLevel/DamageSystem/E_DamageResponseType Enum" :default "NewEnumerator0")))

(event `On Damage Blocked`)

(fn `ApplyBuff`
  (params (Buff :type "/Game/Base/CombatLevel/DamageSystem/S_Buff Structure"))
  (returns (BuffApplied :type Boolean))
  (return false))

(fn `ApplyDebuff`
  (params (Debuff :type "/Game/Base/CombatLevel/DamageSystem/S_Debuff Structure"))
  (returns (DebuffApplied :type Boolean))
  (bind _debuffapplied (`/Game/Base/CombatLevel/DamageSystem/BPC_DamageSystem.ReceiveDebuff` (`self.BPC_DamageSystem`) Debuff))
  (return _debuffapplied))

(fn `GetCurrentHealth`
  (returns (Health :type "Float (double-precision)"))
  (return (`/Game/Base/CombatLevel/DamageSystem/BPC_DamageSystem.Health` (`self.BPC_DamageSystem`))))

(fn `GetFaction`
  (returns (UnitsFaction :type "/Game/Base/CombatLevel/CommandSystem/E_Faction Enum"))
  (return (`self.EFaction`)))

(fn `GetMaxHealth`
  (returns (MaxHealth :type "Float (double-precision)"))
  (return (`/Game/Base/CombatLevel/DamageSystem/BPC_DamageSystem.MaxHealth` (`self.BPC_DamageSystem`))))

(fn `Heal`
  (params (HealAmount :type "Float (double-precision)"))
  (returns (NewHealth :type "Float (double-precision)"))
  (bind _newhealth (`/Game/Base/CombatLevel/DamageSystem/BPC_DamageSystem.Heal` (`self.BPC_DamageSystem`) HealAmount))
  (`/Game/Base/CombatLevel/UI/UWB_UnitHealthBar.UpdateHealth` (`self.HealthBarRef`) _newhealth)
  (return _newhealth))

(fn `HideAbilities`
  (returns (WasSuccessful :type Boolean))
  (bind _cachedcommanduwb (`self.CachedCommandUWB`))
  (`/Engine/EditorBlueprintResources/StandardMacros.IsValid` _cachedcommanduwb
    (:`Is Valid`
      (`Widget.RemoveFromParent` _cachedcommanduwb)
      (return true))
    (:`Is Not Valid`
      (return false))))

(fn `HideHealthBar`
  (returns (WasSuccessful :type Boolean))
  (`SceneComponent.SetVisibility` (`self.HealthBar`) false false)
  (`KismetSystemLibrary.K2_ClearAndInvalidateTimerHandle` (`self.HBRoationTickTimerRef`))
  (return true))

(fn `HideSelectedIndicator`
  (returns (WasSuccessful :type Boolean))
  (bind _selectedindicatorwidget (`self.SelectedIndicatorWidget`))
  (`SceneComponent.SetVisibility` _selectedindicatorwidget false false)
  (`ActorComponent.Deactivate` _selectedindicatorwidget)
  (return true))

(fn `InitHealthBar`
  (bind _bpc_damagesystem (`self.BPC_DamageSystem`))
  (bind _asuwb_unit_health_bar (cast `/Game/Base/CombatLevel/UI/UWB_UnitHealthBar` (`WidgetComponent.GetUserWidgetObject` (`self.HealthBar`))))
  (bind _output_get (set `self.HealthBarRef` _asuwb_unit_health_bar))
  (`/Game/Base/CombatLevel/UI/UWB_UnitHealthBar.UpdateHealth` _output_get (`/Game/Base/CombatLevel/DamageSystem/BPC_DamageSystem.Health` _bpc_damagesystem))
  (`/Game/Base/CombatLevel/UI/UWB_UnitHealthBar.UpdateMaxHealth` _output_get (`/Game/Base/CombatLevel/DamageSystem/BPC_DamageSystem.MaxHealth` _bpc_damagesystem)))

(fn `MoveToLocation`
  (params (Destination :type "Vector Structure"))
  (returns (WasSuccessful :type Boolean))
  (`AIBlueprintHelperLibrary.SimpleMoveToLocation` (`self.GetController`) Destination)
  (return true))

(fn `ShowAbilities`
  (returns (WasSuccessful :type Boolean))
  (if (not (`/Game/Base/CombatLevel/DamageSystem/BPC_DamageSystem.IsDead` (`self.BPC_DamageSystem`)))
    (bind _returnvalue (`|CreateWidget` "/Game/Base/CombatLevel/UI/UWB_UnitCommandBar.UWB_UnitCommandBar_C" (`GameplayStatics.GetPlayerController` 0)))
    (bind _output_get (set `self.CachedCommandUWB` _returnvalue))
    (`/Engine/EditorBlueprintResources/StandardMacros.IsValid` _output_get
      (:`Is Valid`
        (`UserWidget.AddToViewport` _returnvalue 0)
        (`WidgetBlueprintLibrary.SetInputMode_GameAndUIEx` (`GameplayStatics.GetPlayerController` 0) null "LockAlways" false)
        (return true))
      (:`Is Not Valid`
        _)))
  (return false))

(fn `ShowHealthBar`
  (returns (WasSuccessful :type Boolean))
  (bind _hbrotationtickrate (`self.HBRotationTickRate`))
  (bind _returnvalue (`KismetSystemLibrary.K2_SetTimerDelegate` (`|CreateDelegate` :!event `UpdateHealthBarWidgetRotation`) _hbrotationtickrate true _hbrotationtickrate))
  (set `self.HBRoationTickTimerRef` _returnvalue)
  (`SceneComponent.SetVisibility` (`self.HealthBar`) true false)
  (return true))

(fn `ShowSelectedIndicator`
  (returns (WasSuccessful :type Boolean))
  (bind _selectedindicatorwidget (`self.SelectedIndicatorWidget`))
  (`ActorComponent.Activate` _selectedindicatorwidget false)
  (`SceneComponent.SetVisibility` _selectedindicatorwidget true false)
  (return true))

(fn `TakeDamage`
  (params (Damage :type "/Game/Base/CombatLevel/DamageSystem/S_Damage Structure"))
  (returns (WasDamaged :type Boolean))
  (bind _bpc_damagesystem (`self.BPC_DamageSystem`))
  (bind _damageapplied (`/Game/Base/CombatLevel/DamageSystem/BPC_DamageSystem.TakeDamage` _bpc_damagesystem Damage))
  (if _damageapplied
    (`/Game/Base/CombatLevel/UI/UWB_UnitHealthBar.UpdateHealth` (`self.HealthBarRef`) (`/Game/Base/CombatLevel/DamageSystem/BPC_DamageSystem.Health` _bpc_damagesystem))
    (return _damageapplied)
    (else
      (return false))))

(fn `UserConstructionScript`
  (bind _bpc_damagesystem (`self.BPC_DamageSystem`))
  (`|ExecutionSequence`
    (:`then_0`
      (add `/Game/Base/CombatLevel/DamageSystem/BPC_DamageSystem.OnDeath` _bpc_damagesystem (`|CreateDelegate` :!event `On Death`)))
    (:`then_1`
      (add `/Game/Base/CombatLevel/DamageSystem/BPC_DamageSystem.OnDamageResponse` _bpc_damagesystem (`|CreateDelegate` :!event `On Damage Response`)))
    (:`then_2`
      (add `/Game/Base/CombatLevel/DamageSystem/BPC_DamageSystem.OnBlocked` _bpc_damagesystem (`|CreateDelegate` :!event `On Damage Blocked`)))))